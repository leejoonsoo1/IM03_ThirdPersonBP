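; Player character with camera-relative movement, sprint, a jump-based evade and a one-handed sword attack.
; BeginPlay spawns BP_OneHand at the holster socket; separate events move it between hand and holster.
; Toggling the weapon locks movement and switches between controller-yaw and movement-oriented rotation, until externally triggered completion events restore movement and set Drawn.
; Drawn gates the attack montage, and an Attacking flag blocks repeats until EndAction clears it.
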(event `InputAction|Action`
  (params (Key :type "Key Structure"))
  (:`Pressed`
    (if (`self.bDrawn`)
      (if (not (`self.bAttacking`))
        (set `self.bAttacking` true)
        (`self.PlayAnimMontage` "/Game/Character/Animations/OneHand/Sword_Attack_1_Montage.Sword_Attack_1_Montage")))))

(event `EndAction`
  (set `self.bAttacking` false))

(event `InputAxis|Turn`
  (params (AxisValue :type "Float (single-precision)"))
  (`self.AddControllerYawInput` AxisValue))

(event `InputAxis|Lookup`
  (params (AxisValue :type "Float (single-precision)"))
  (`self.AddControllerPitchInput` AxisValue))

(event `InputAxis|MoveForward`
  (params (AxisValue :type "Float (single-precision)"))
  (bind (_returnvalue_roll _returnvalue_pitch _returnvalue_yaw) (`KismetMathLibrary.BreakRotator` (`self.GetControlRotation`)))
  (if (`self.bCanMove`)
    (`self.AddMovementInput` (`KismetMathLibrary.GetForwardVector` (`KismetMathLibrary.MakeRotator` 0.0 0.0 _returnvalue_yaw)) AxisValue)))

(event `InputAxis|MoveRight`
  (params (AxisValue :type "Float (single-precision)"))
  (bind (_returnvalue_roll _returnvalue_pitch _returnvalue_yaw) (`KismetMathLibrary.BreakRotator` (`self.GetControlRotation`)))
  (if (`self.bCanMove`)
    (`self.AddMovementInput` (`KismetMathLibrary.GetRightVector` (`KismetMathLibrary.MakeRotator` 0.0 0.0 _returnvalue_yaw)) AxisValue)))

(event `InputAction|Sprint`
  (params (Key :type "Key Structure"))
  (bind _charactermovement (`self.CharacterMovement`))
  (:`Pressed`
    (set `CharacterMovementComponent.MaxWalkSpeed` 600.0 _charactermovement))
  (:`Released`
    (set `CharacterMovementComponent.MaxWalkSpeed` 400.0 _charactermovement)))

(event `InputAction|Evade`
  (params (Key :type "Key Structure"))
  (:`Pressed`
    (`self.Jump`))
  (:`Released`
    (`self.StopJumping`)))

(event `InputAction|OneHand`
  (params (Key :type "Key Structure"))
  (:`Pressed`
    (if (`self.bDrawn`)
      (`self.UnequipOneHand`)
      (else
        (`self.EquipOneHand`)))))

(event `EquippedOneHand`
  (set `self.bEquipping` false)
  (set `self.bCanMove` true)
  (set `self.bCanMove` true)
  (set `self.bDrawn` true))

(event `EquipOneHand`
  (set `self.bEquipping` true)
  (set `self.bUseControllerRotationYaw` true)
  (set `CharacterMovementComponent.bOrientRotationToMovement` false (`self.CharacterMovement`))
  (set `self.bCanMove` false))

(event `UnequipOneHand`
  (set `self.bUnequipping` true)
  (set `self.bUseControllerRotationYaw` false)
  (set `CharacterMovementComponent.bOrientRotationToMovement` true (`self.CharacterMovement`))
  (set `self.bCanMove` false))

(event `UnEquippedOneHand`
  (set `self.bUnequipping` false)
  (set `self.bCanMove` true)
  (set `self.bDrawn` false))

(event `AttachOneHand`
  (`self.K2_AttachToComponent` (`self.OneHand`) (`self.Mesh`) "Hand_Sword" "KeepRelative" "KeepRelative" "KeepRelative" true))

(event `DetachOneHand`
  (`self.K2_AttachToComponent` (`self.OneHand`) (`self.Mesh`) "Holster_Sword" "KeepRelative" "KeepRelative" "KeepRelative" true))

(event `self.ReceiveBeginPlay`
  (bind _returnvalue (`|SpawnActorFromClass` "/Game/Weapons/BP_OneHand.BP_OneHand_C" (`KismetMathLibrary.MakeTransform` (0.0 0.0 0.0)) "Undefined" "OverrideRootScale" self null))
  (bind _output_get (set `self.OneHand` _returnvalue))
  (`self.K2_AttachToComponent` _output_get (`self.Mesh`) "Holster_Sword" "KeepRelative" "KeepRelative" "KeepRelative" true))

(fn `UserConstructionScript`)