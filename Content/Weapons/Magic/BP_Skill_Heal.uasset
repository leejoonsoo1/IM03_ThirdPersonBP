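; BP_Skill_Heal is a magic skill Blueprint for a heal spell, built on a parent skill class that supplies the casting flow.
; When the spell starts, it runs the parent logic, disables the owner's movement through its magic interface and plays a buff montage on the owning character.
; When the cast finishes, it runs the parent logic and re-enables movement; no healing logic appears in this Blueprint itself.
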(event `self.Spell`
  (`parent.Spell`)
  (`/Game/Weapons/BP_Weapon.SetStateMove` (`self.GetOwnerToMagic`) false)
  (`Character.PlayAnimMontage` (`self.GetOwnerToCharacter`) "/Game/Character/Animations/Magic/MG_Buff_Montage.MG_Buff_Montage" 1.0 "None"))

(event `self.Spelled`
  (`parent.Spelled`)
  (`/Game/Weapons/BP_Weapon.SetStateMove` (`self.GetOwnerToMagic`) true))

(fn `UserConstructionScript`
  (`parent.UserConstructionScript`))