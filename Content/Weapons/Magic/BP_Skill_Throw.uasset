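; Throwable magic skill that shows a hand particle effect and toggles the owning BP_Player's aim mode when set or unset.
; A Throws array pairs projectile classes with hand particles, and ChangeProjectile selects the active entry by class.
; Spell plays the fireball montage, while the separate DoThrow event spawns the active projectile ahead of the player camera, oriented by control rotation.
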(event `self.ReceiveBeginPlay`
  (bind (_output_projectileclass _output_handparticle) (break `/Game/Structs/FThrowData` (`|GetArrayItem` (`self.Throws`) (`self.ThrowIndex`))))
  (`ParticleSystemComponent.SetTemplate` (`self.ParticleSystem`) _output_handparticle)
  (`SceneComponent.SetVisibility` (`self.ParticleSystem`) false false)
  (switch `int` (`self.ThrowIndex`)
    (:`0`
      (`SceneComponent.SetRelativeScale3D` (`self.ParticleSystem`) (0.2 0.2 0.2)))
    (:`1`
      (`SceneComponent.SetRelativeScale3D` (`self.ParticleSystem`) (0.2 0.2 0.2)))))

(event `self.OnSet`
  (`parent.OnSet`)
  (`SceneComponent.SetVisibility` (`self.ParticleSystem`) true false)
  (bind _asbp_player (cast `/Game/Player/BP_Player` (`self.GetOwnerToCharacter`)))
  (`/Game/Player/BP_Player.OnAim` _asbp_player))

(event `self.OnUnset`
  (`parent.OnUnset`)
  (`SceneComponent.SetVisibility` (`self.ParticleSystem`) false false)
  (bind _asbp_player (cast `/Game/Player/BP_Player` (`self.GetOwnerToCharacter`)))
  (`/Game/Player/BP_Player.OffAim` _asbp_player))

(event `self.Spell`
  (`parent.Spell`)
  (`Character.PlayAnimMontage` (`self.GetOwnerToCharacter`) "/Game/Character/Animations/Magic/MG_Fireball_03_Montage.MG_Fireball_03_Montage" 1.0 "None"))

(event `self.Spelled`
  (`parent.Spelled`))

(event `DoThrow`
  (bind _output_projectileclass (break `/Game/Structs/FThrowData` (`|GetArrayItem` (`self.Throws`) (`self.ThrowIndex`))))
  (`|SpawnActorFromClass` _output_projectileclass (`KismetMathLibrary.MakeTransform` (`self.GetViewPoint`) (`Pawn.GetControlRotation` (`self.GetOwnerToCharacter`))) "Undefined" "OverrideRootScale" self null))

(fn `ChangeProjectile`
  (params (NewClass :type "/Game/Weapons/Magic/BP_Projectile Class Reference"))
  (locals (It :type Integer))
  (bind _output_projectileclass (break `/Game/Structs/FThrowData` (`|GetArrayItem` (`self.Throws`) (`local.It`))))
  (bind (_output_projectileclass_2 _output_handparticle) (break `/Game/Structs/FThrowData` (`|GetArrayItem` (`self.Throws`) (`self.ThrowIndex`))))
  (for (_ _array_index) (`self.Throws`)
    (set `local.It` _array_index)
    (if (== _output_projectileclass (`local.NewClass`))
      (break)))
  (set `self.ThrowIndex` (`local.It`))
  (`ParticleSystemComponent.SetTemplate` (`self.ParticleSystem`) _output_handparticle))

(fn `GetViewPoint`
  (returns (ReturnValue :type "Vector Structure"))
  (bind _asbp_player (cast `/Game/Player/BP_Player` (`self.GetOwnerToCharacter`)))
  (bind _camera (`/Game/Player/BP_Player.Camera` _asbp_player))
  (return (+ (`SceneComponent.K2_GetComponentLocation` _camera) (* (`SceneComponent.GetForwardVector` _camera) 380.0))))

(fn `UserConstructionScript`
  (`parent.UserConstructionScript`))