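; Magic weapon that casts skill actors in place of a regular attack.
; On BeginPlay it spawns Heal, Warp and Throw skills, attaches each to the owning Character's mesh, and hard-sets Throw as the current skill.
; Attack enters the spelling state and calls Spell on the current skill when valid and able to attack; EndAction returns to idle and calls Spelled.
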(event `self.EndAction`
  (`parent.EndAction`)
  (`self.SetStateIdling`)
  (`/Game/Weapons/Magic/BP_Skill.Spelled` (`self.CurrentSkill`)))

(event `self.Attack`
  (bind _currentskill (`self.CurrentSkill`))
  (`parent.Attack`)
  (if (and (`KismetSystemLibrary.IsValid` _currentskill) (`self.CanAttack`))
    (`self.SetStateSpelling`)
    (`/Game/Weapons/Magic/BP_Skill.Spell` _currentskill)))

(event `self.ReceiveBeginPlay`
  (`parent.ReceiveBeginPlay`)
  (`|ExecutionSequence`
    (:`then_0`
      (bind _returnvalue (`|SpawnActorFromClass` "/Game/Weapons/Magic/BP_Skill_Heal.BP_Skill_Heal_C" (`KismetMathLibrary.MakeTransform` (0.0 0.0 0.0)) "Undefined" "OverrideRootScale" self null))
      (set `self.Heal` _returnvalue)
      (bind _ascharacter (cast `Character` (`self.GetOwner`)))
      (`self.K2_AttachToComponent` (`self.Heal`) (`Character.Mesh` _ascharacter) "None" "KeepRelative" "KeepRelative" "KeepRelative" true))
    (:`then_1`
      (bind _returnvalue_2 (`|SpawnActorFromClass` "/Game/Weapons/Magic/BP_Skill_Warp.BP_Skill_Warp_C" (`KismetMathLibrary.MakeTransform` (0.0 0.0 0.0)) "Undefined" "OverrideRootScale" self null))
      (set `self.Warp` _returnvalue_2)
      (bind _ascharacter_2 (cast `Character` (`self.GetOwner`)))
      (`self.K2_AttachToComponent` (`self.Warp`) (`Character.Mesh` _ascharacter_2) "None" "KeepRelative" "KeepRelative" "KeepRelative" true))
    (:`then_2`
      (bind _returnvalue_3 (`|SpawnActorFromClass` "/Game/Weapons/Magic/BP_Skill_Throw.BP_Skill_Throw_C" (`KismetMathLibrary.MakeTransform` (0.0 0.0 0.0)) "Undefined" "OverrideRootScale" self null))
      (set `self.Throw` _returnvalue_3)
      (bind _ascharacter_3 (cast `Character` (`self.GetOwner`)))
      (`self.K2_AttachToComponent` (`self.Throw`) (`Character.Mesh` _ascharacter_3) "None" "KeepRelative" "KeepRelative" "KeepRelative" true))
    (:`then_3`
      ;[1 1 1] 현재 워프만 가능
      (set `self.CurrentSkill` (`self.Throw`)))))

(fn `UserConstructionScript`
  (`parent.UserConstructionScript`))