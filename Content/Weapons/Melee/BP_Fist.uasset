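; BP_Fist is an unarmed melee weapon that provides punch and kick hit detection for the character that owns it.
; On BeginPlay it attaches left and right punch and kick collisions to matching Fist sockets on the owning Character's mesh.
; Overlaps on the Capsule component send a fixed damage amount to the other actor.
; Collision on/off events defer entirely to the parent class.
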(event `self.Capsule.OnComponentBeginOverlap`
  (params (OverlappedComponent :type "PrimitiveComponent Object Reference") (OtherActor :type "Actor Object Reference") (OtherComp :type "PrimitiveComponent Object Reference") (OtherBodyIndex :type Integer) (bFromSweep :type Boolean) (SweepResult :type "HitResult Structure (by ref)"))
  (`self.SendDamage` OtherActor 10.0))

(event `self.ReceiveBeginPlay`
  (`parent.ReceiveBeginPlay`)
  (`|ExecutionSequence`
    (:`then_0`
      (`self.AttachCollisionToSocket` (`self.LeftPunch`) "Fist_LeftPunch")
      (`self.AttachCollisionToSocket` (`self.RightPunch`) "Fist_RightPunch"))
    (:`then_1`
      (`self.AttachCollisionToSocket` (`self.LeftKick`) "Fist_LeftKick")
      (`self.AttachCollisionToSocket` (`self.RightKick`) "Fist_RightKick"))))

(event `self.OnCollision`
  (`parent.OnCollision`))

(event `self.OffCollsion`
  (`parent.OffCollsion`))

(fn `AttachCollisionToSocket`
  (params (Collision :type "SphereComponent Object Reference") (SocketName :type Name))
  (bind _ascharacter (cast `Character` (`self.GetOwner`)))
  (`SceneComponent.K2_AttachToComponent` (`local.Collision`) (`Character.Mesh` _ascharacter) (`local.SocketName`) "KeepRelative" "KeepRelative" "KeepRelative" true))

(fn `UserConstructionScript`)