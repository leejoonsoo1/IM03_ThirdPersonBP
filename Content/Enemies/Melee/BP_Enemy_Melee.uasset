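; Melee enemy Blueprint that carries a two-handed greatsword and extends its parent's weapon handling.
; Attach and Detach move the TwoHand component between the hand and holster sockets on the mesh and track the state in OnHanded.
; Equipped and Unequipped switch CombatType and set or clear the active weapon object.
; Each event calls the parent implementation first, and the construction script only runs the parent's.
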(event `self.Attach`
  (`parent.Attach`)
  (`self.K2_AttachToComponent` (`self.TwoHand`) (`self.Mesh`) "Hand_GreatSword" "KeepRelative" "KeepRelative" "KeepRelative" true)
  (set `self.bOnHanded` true))

(event `self.Detach`
  (`parent.Detach`)
  (`self.K2_AttachToComponent` (`self.TwoHand`) (`self.Mesh`) "Holster_GreatSword" "KeepRelative" "KeepRelative" "KeepRelative" true)
  (set `self.bOnHanded` false))

(event `self.Equipped`
  (`parent.Equipped`)
  (set `self.CombatType` "NewEnumerator1")
  (`self.SetWeaponObject` (`self.TwoHand`)))

(event `self.Unequipped`
  (`parent.Unequipped`)
  (set `self.CombatType` "NewEnumerator0")
  (`self.SetWeaponObject` null))

(fn `UserConstructionScript`
  (`parent.UserConstructionScript`))