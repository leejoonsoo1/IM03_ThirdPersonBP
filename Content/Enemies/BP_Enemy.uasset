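; Enemy character that spawns a two-handed weapon in its hand and reacts to damage.
; Each hit lowers StatusComponent health, which updates the health widget, shows damage text, plays a montage, faces the attacker and flashes red.
; Death triggers an impulse-driven ragdoll and delayed destruction; surviving a magic throw can briefly activate a hit effect.
; Weapon and state interface functions are mostly stubs, and the melee hit branch is empty.
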(event `self.ReceiveBeginPlay`
  (bind _returnvalue (`|SpawnActorFromClass` "/Game/Weapons/Melee/BP_TwoHand.BP_TwoHand_C" (`KismetMathLibrary.MakeTransform` (0.0 0.0 0.0)) "Undefined" "OverrideRootScale" self null))
  (bind _output_get (set `self.TwoHand` _returnvalue))
  (`self.K2_AttachToComponent` _output_get (`self.Mesh`) "Hand_GreatSword" "KeepRelative" "KeepRelative" "KeepRelative" true))

(event `self.ReceiveAnyDamage`
  (params (Damage :type "Float (single-precision)") (DamageType :type "DamageType Object Reference") (InstigatedBy :type "Controller Object Reference") (DamageCauser :type "Actor Object Reference"))
  (set `self.Causer` DamageCauser)
  (bind _ascharacter (cast `Character` (`Controller.K2_GetPawn` InstigatedBy)))
  (set `self.Attacker` _ascharacter)
  (bind _output_get (set `self.Damage` Damage))
  (`/Game/Components/StatusComponent.DecreaseHealth` (`self.StatusComponent`) _output_get)
  (bind _returnvalue (`|CreateWidget` "/Game/UI/WB_DamageText.WB_DamageText_C" null self (`self.Damage`)))
  (`UserWidget.AddToViewport` _returnvalue 0)
  (`self.PlayAnimMontage` "/Game/Character/Animations/Common/HitReaction_Montage.HitReaction_Montage" 3.0)
  (`self.K2_SetActorRotation` (`KismetMathLibrary.FindLookAtRotation` (`self.K2_GetActorLocation`) (`self.K2_GetActorLocation` (`self.Attacker`))))
  (`MeshComponent.SetVectorParameterValueOnMaterials` (`self.Mesh`) "BodyColor" (1.0 0.0 0.0))
  (`KismetSystemLibrary.Delay` 0.1)
  (`MeshComponent.SetVectorParameterValueOnMaterials` (`self.Mesh`) "BodyColor" (`KismetMathLibrary.Conv_LinearColorToVector` (`self.BodyColor`)))
  (if (`/Game/Components/StatusComponent.IsDead` (`self.StatusComponent`))
    (if (`|EnumInequality` (`self.StateType`) "NewEnumerator4")
      (set `self.StateType` "NewEnumerator4")
      (`self.Ragdoll`)
      (`KismetSystemLibrary.Delay` 5.0)
      (`self.EndDead`))
    (else
      (bind _asbp_magic (cast `/Game/Weapons/Magic/BP_Magic` (`self.Causer`))
        (:`then`
          (bind _asbp_skill_throw (cast `/Game/Weapons/Magic/BP_Skill_Throw` (`/Game/Weapons/Magic/BP_Magic.CurrentSkill` _asbp_magic)))
          (switch `int` (`/Game/Weapons/Magic/BP_Skill_Throw.ThrowIndex` _asbp_skill_throw)
            (:`0`
              (`ActorComponent.SetActive` (`self.HitEffect`) true false)
              (`KismetSystemLibrary.Delay` 3.0)
              (`ActorComponent.SetActive` (`self.HitEffect`) false false))))
        (:`CastFailed`
          (bind _asbp_melee (cast `/Game/Weapons/Melee/BP_Melee` (`self.Causer`)))
          (switch `/Game/Enums/EMeleeType` (`/Game/Weapons/Melee/BP_Melee.MeleeType` _asbp_melee)))))))

(event `EndDead`
  (`self.K2_DestroyActor` (`self.TwoHand`))
  (`self.K2_DestroyActor`))

(event `self.StatusComponent.OnHealthChanged`
  (params (NewHealth :type "Float (single-precision)") (MaxHealth :type "Float (single-precision)"))
  (bind _aswb_enemy_health (cast `/Game/UI/WB_EnemyHealth` (`WidgetComponent.GetUserWidgetObject` (`self.HealthWidget`))))
  (`/Game/UI/WB_EnemyHealth.UpdateHealthBar` _aswb_enemy_health NewHealth MaxHealth))

(fn `Attach`)

(fn `Detach`)

(fn `Equipped`)

(fn `GetWeaponCombatType`
  (returns (CurrentCombatType :type "/Game/Enums/ECombatType Enum"))
  (return "NewEnumerator0"))

(fn `GetWeaponObject`
  (returns (CurrentWeapon :type "/Game/Weapons/BP_Weapon Object Reference"))
  (return null))

(fn `IsStateAttacking`
  (returns (NewParam :type Boolean))
  (return false))

(fn `IsStateIdling`
  (returns (NewParam :type Boolean))
  (return false))

(fn `Ragdoll`
  (bind _mesh (`self.Mesh`))
  (`PrimitiveComponent.SetCollisionEnabled` (`self.CapsuleComponent`) "NoCollision")
  (`PrimitiveComponent.SetSimulatePhysics` _mesh true)
  (`PrimitiveComponent.SetCollisionProfileName` _mesh "Ragdoll" true)
  (`PrimitiveComponent.AddForce` _mesh (* (* (`KismetMathLibrary.GetDirectionUnitVector` (`self.K2_GetActorLocation` (`self.Attacker`)) (`self.K2_GetActorLocation`)) (`self.Damage`)) 250000) "None" false))

(fn `SetStateAttacking`
  (returns (NewParam :type Boolean))
  (return false))

(fn `SetStateIdling`
  (returns (NewParam :type Boolean))
  (return false))

(fn `SetStateMove`
  (params (bMove :type Boolean))
  (returns (NewParam1 :type Boolean))
  (return false))

(fn `SetStateSpelling`
  (returns (NewParam :type Boolean))
  (return false))

(fn `SetWeaponObject`
  (params (NewWeapon :type "/Game/Weapons/BP_Weapon Object Reference"))
  (returns (Weapon :type "/Game/Weapons/BP_Weapon Object Reference"))
  (return null))

(fn `UnEquipped`
  (set `self.StateType` "NewEnumerator0"))

(fn `UserConstructionScript`
  (`MeshComponent.SetVectorParameterValueOnMaterials` (`self.Mesh`) "BodyColor" (`KismetMathLibrary.Conv_LinearColorToVector` (`self.BodyColor`)))
  (`TextRenderComponent.K2_SetText` (`self.PawnName`) (`KismetTextLibrary.Conv_StringToText` (`KismetSystemLibrary.GetDisplayName` self))))

(fn `WeaponAttach`
  (returns (NewParam :type Boolean))
  (`self.Attach`)
  (return false))

(fn `WeaponDetach`
  (returns (NewParam :type Boolean))
  (`self.Detach`)
  (return false))

(fn `WeaponEquipped`
  (returns (NewParam :type Boolean))
  (`self.Equipped`)
  (return false))

(fn `WeaponUnEquipped`
  (returns (NewParam :type Boolean))
  (`self.UnEquipped`)
  (return false))